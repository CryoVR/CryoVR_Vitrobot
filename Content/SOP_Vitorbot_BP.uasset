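; SOP_Vitorbot_BP is an actor with a swinging door that a VR motion controller toggles by touch.
; An overlap of Door_Collider by a TP_MotionController starts the rotation.
; Tick turns the door by a fixed, frame-rate-dependent step, then stops it and flips its direction once yaw passes the open or closed limit of a quarter turn.
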(event `self.ReceiveTick`
  (params (DeltaSeconds :type "Float (single-precision)"))
  (bind _door (`self.Door`))
  (bind (_relativerotation_roll _relativerotation_pitch _relativerotation_yaw) (`KismetMathLibrary.BreakRotator` (`SceneComponent.RelativeRotation` (`self.Door`))))
  (bind (_relativerotation_roll_2 _relativerotation_pitch_2 _relativerotation_yaw_2) (`KismetMathLibrary.BreakRotator` (`SceneComponent.RelativeRotation` (`self.Door`))))
  (if (`self.Is_Door_Rotating`)
    (if (`self.Is_Door_Opening`)
      (`SceneComponent.K2_AddRelativeRotation` _door (struct :`Yaw` 3.0) false false)
      (else
        (`SceneComponent.K2_AddRelativeRotation` _door (struct :`Yaw` -3.0) false false)))
    (if (> _relativerotation_yaw_2 90.0)
      (set `self.Is_Door_Opening` false)
      (set `self.Is_Door_Rotating` false)
      (elif (<= _relativerotation_yaw 0.0)
        (set `self.Is_Door_Opening` true)
        (set `self.Is_Door_Rotating` false)))))

(event `self.ReceiveActorBeginOverlap`
  (params (OtherActor :type "Actor Object Reference")))

(event `self.Door_Collider.OnComponentBeginOverlap`
  (params (OverlappedComponent :type "PrimitiveComponent Object Reference") (OtherActor :type "Actor Object Reference") (OtherComp :type "PrimitiveComponent Object Reference") (OtherBodyIndex :type Integer) (bFromSweep :type Boolean) (SweepResult :type "HitResult Structure (by ref)"))
  (cast `TP_MotionController` OtherActor)
  (set `self.Is_Door_Rotating` true))

(fn `UserConstructionScript`)