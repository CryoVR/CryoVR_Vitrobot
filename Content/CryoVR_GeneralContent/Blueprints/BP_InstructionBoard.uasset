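; BP_InstructionBoard is an in-world board actor that shows instruction text and a status description on text components.
; AddInstruction fills three lines in rotation, clearing the board when it wraps to the first, while SetInstruction clears it and reveals three lines at two-second intervals.
; Separately, Tick looks up the current Status in the Global_Arrays game instance's IndexDescriptions map and writes any match to a status line.
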(event `self.ReceiveBeginPlay`
  (bind _asglobal_arrays (cast `/Game/CryoVR_GeneralContent/Blueprints/Global_Arrays` (`GameplayStatics.GetGameInstance`)))
  (set `self.As Global Arrays` _asglobal_arrays))

(event `self.ReceiveTick`
  (params (DeltaSeconds :type "Float (single-precision)"))
  (bind _as_global_arrays (`self.As Global Arrays`))
  (bind (_value _returnvalue) (`BlueprintMapLibrary.Map_Find` (`/Game/CryoVR_GeneralContent/Blueprints/Global_Arrays.Index & Descriptions` _as_global_arrays) (`/Game/CryoVR_GeneralContent/Blueprints/Global_Arrays.Status` _as_global_arrays)))
  (if _returnvalue
    (`TextRenderComponent.K2_SetText` (`self.TR_05`) (`KismetTextLibrary.Conv_StringToText` _value))))

(event `ClearBoard`
  ;[1 1 1] Clear all the instructions
  (bind _output_get (set `self.description` ""))
  (`TextRenderComponent.K2_SetText` (`self.TR_01`) _output_get)
  (`TextRenderComponent.K2_SetText` (`self.TR_02`) _output_get)
  (`TextRenderComponent.K2_SetText` (`self.TR_03`) _output_get)
  (set `self.nextLineIndex` 0))

(event `AddInstruction`
  (params (instruction :type Text))
  ;[1 1 1] Add a instruction in the next line
  (switch `int` (`self.nextLineIndex`)
    (:`0`
      (`self.ClearBoard`)
      (bind _output_get (set `self.description` instruction))
      (`TextRenderComponent.K2_SetText` (`self.TR_01`) _output_get)
      (set `self.nextLineIndex` 1))
    (:`1`
      (bind _output_get_2 (set `self.description` instruction))
      (`TextRenderComponent.K2_SetText` (`self.TR_02`) _output_get_2)
      (set `self.nextLineIndex` 2))
    (:`2`
      (bind _output_get_3 (set `self.description` instruction))
      (`TextRenderComponent.K2_SetText` (`self.TR_03`) _output_get_3)
      (set `self.nextLineIndex` 0))))

(event `SetInstruction`
  (params (Instruction1 :type String) (Instruction2 :type String) (Instruction3 :type String))
  ;[1 1 1] Set the instructions
  (`self.ClearBoard`)
  (bind _output_get (set `self.description` (`KismetTextLibrary.Conv_StringToText` Instruction1)))
  (`TextRenderComponent.K2_SetText` (`self.TR_01`) _output_get)
  (`KismetSystemLibrary.Delay` 2.0)
  (bind _output_get_2 (set `self.description` (`KismetTextLibrary.Conv_StringToText` Instruction2)))
  (`TextRenderComponent.K2_SetText` (`self.TR_02`) _output_get_2)
  (`KismetSystemLibrary.Delay` 2.0)
  (bind _output_get_3 (set `self.description` (`KismetTextLibrary.Conv_StringToText` Instruction3)))
  (`TextRenderComponent.K2_SetText` (`self.TR_03`) _output_get_3)
  (set `self.nextLineIndex` 0))

(fn `UserConstructionScript`)