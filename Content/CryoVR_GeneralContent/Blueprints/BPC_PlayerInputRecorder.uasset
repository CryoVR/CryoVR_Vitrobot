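; Actor component that records VR player input, likely for later playback, into the GameRecord map on the Global_Arrays game instance.
; A looping timer calls RecordInput at a fixed delta, storing hand controller transforms, grip states and camera transform keyed by an accumulated time.
; Events start (clearing prior records), continue from a given time, stop, or clear the recording.
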(event `self.ReceiveBeginPlay`
  (bind _asglobal_arrays (cast `/Game/CryoVR_GeneralContent/Blueprints/Global_Arrays` (`GameplayStatics.GetGameInstance`)))
  (set `self.As Global Arrays` _asglobal_arrays))

(event `StartRecording`
  (`self.ClearRecords`)
  (`KismetSystemLibrary.K2_SetTimer` self "RecordInput" (`self.recordDeltaTime`) true))

(event `ContinueRecording`
  (params (StartTime :type "Float (double-precision)"))
  (set `self.globalTime` StartTime)
  (`KismetSystemLibrary.K2_SetTimer` self "RecordInput" (`self.recordDeltaTime`) true))

(event `EndRecording`
  (`KismetSystemLibrary.K2_ClearTimer` self "RecordInput"))

(event `ClearRecords`
  (`BlueprintMapLibrary.Map_Clear` (`/Game/CryoVR_GeneralContent/Blueprints/Global_Arrays.Game_Record` (`self.As Global Arrays`))))

(fn `RecordInput`
  (bind _lefthand (`self.leftHand`))
  (bind _righthand (`self.rightHand`))
  (`BlueprintMapLibrary.Map_Add` (`/Game/CryoVR_GeneralContent/Blueprints/Global_Arrays.Game_Record` (`self.As Global Arrays`)) (`self.globalTime`) (make `/Game/CryoVR_GeneralContent/Blueprints/S_InputTick` (`SceneComponent.K2_GetComponentToWorld` (`/Game/VirtualRealityBP/Blueprints/BP_MotionController.MotionController` _lefthand)) (`/Game/VirtualRealityBP/Blueprints/BP_MotionController.bWantsToGrip` _lefthand) (`SceneComponent.K2_GetComponentToWorld` (`/Game/VirtualRealityBP/Blueprints/BP_MotionController.MotionController` _righthand)) (`/Game/VirtualRealityBP/Blueprints/BP_MotionController.bWantsToGrip` _righthand) (`SceneComponent.K2_GetComponentToWorld` (`self.camera`))))
  (set `self.globalTime` (+ (`self.globalTime`) (`self.recordDeltaTime`))))