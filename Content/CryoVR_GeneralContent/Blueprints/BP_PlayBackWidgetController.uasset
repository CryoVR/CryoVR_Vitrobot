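; VR control panel actor for session replay, showing playback time and speed on a UI_Replay_Controller widget.
; Tick feeds the widget from the Player's BPCPlayBackController and advances the step index past each recorded time in Global_Arrays.
; Index-finger overlaps on box triggers pause, resume, slow or speed playback, sharing a half-second input lock.
; Step text, hand-gesture switching and camera-facing logic are disconnected.
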(event `self.ReceiveBeginPlay`
  (bind _asglobal_arrays (cast `/Game/CryoVR_GeneralContent/Blueprints/Global_Arrays` (`GameplayStatics.GetGameInstance`)))
  (set `self.As Global Arrays` _asglobal_arrays)
  (bind _asui_replay_controller (cast `/Game/CryoVR_GeneralContent/UI_Replay_Controller` (`WidgetComponent.GetUserWidgetObject` (`self.Controller_UI`))))
  (set `self.As UI Replay Controller` _asui_replay_controller)
  (`self.SetStep`))

(event `SetStep`)

(event `self.ReceiveTick`
  (params (DeltaSeconds :type "Float (single-precision)"))
  (bind _bpc_playbackcontroller (`/Game/CryoVR_GeneralContent/Blueprints/BP_PlayBackCharacter.BPC_PlayBackController` (`self.Player`)))
  (`|ExecutionSequence`
    (:`then_1`
      ;[1 1 1] Update time and play speed
      (`/Game/CryoVR_GeneralContent/UI_Replay_Controller.SetTime` (`self.As UI Replay Controller`) (`/Game/CryoVR_GeneralContent/Blueprints/BPC_PlayBackController.globalTime` _bpc_playbackcontroller))
      (`/Game/CryoVR_GeneralContent/UI_Replay_Controller.SetSpeed` (`self.As UI Replay Controller`) (`/Game/CryoVR_GeneralContent/Blueprints/BPC_PlayBackController.SpeedFactor` _bpc_playbackcontroller))
      ;[1 1 1] If global time beyond current step time, next time
      (if (> (`/Game/CryoVR_GeneralContent/Blueprints/BPC_PlayBackController.globalTime` (`/Game/CryoVR_GeneralContent/Blueprints/BP_PlayBackCharacter.BPC_PlayBackController` (`self.Player`))) (`|GetArrayItem` (`/Game/CryoVR_GeneralContent/Blueprints/Global_Arrays.User_Time_Array` (`self.As Global Arrays`)) (`self.CurrentStepIndex`)))
        (`/Engine/EditorBlueprintResources/StandardMacros.IncrementInt` (`self.CurrentStepIndex`)
          (:`  `
            (`self.SetStep`)))))))

(event `self.Gesture_Box.OnComponentBeginOverlap`
  (params (OverlappedComponent :type "PrimitiveComponent Object Reference") (OtherActor :type "Actor Object Reference") (OtherComp :type "PrimitiveComponent Object Reference") (OtherBodyIndex :type Integer) (bFromSweep :type Boolean) (SweepResult :type "HitResult Structure (by ref)"))
  ;[1 1 1] Change hand gesture
  (bind _asbp_motion_controller (cast `/Game/VirtualRealityBP/Blueprints/BP_MotionController` OtherActor))
  (if (== (`/Game/VirtualRealityBP/Blueprints/BP_MotionController.IndexFingerColli` _asbp_motion_controller) OtherComp)
    (if (`/Game/VirtualRealityBP/Blueprints/BP_MotionController.bWantsToGrip` _asbp_motion_controller)
      _)))

(event `self.Gesture_Box.OnComponentEndOverlap`
  (params (OverlappedComponent :type "PrimitiveComponent Object Reference") (OtherActor :type "Actor Object Reference") (OtherComp :type "PrimitiveComponent Object Reference") (OtherBodyIndex :type Integer))
  ;[1 1 1] Change hand gesture
  (bind _asbp_motion_controller (cast `/Game/VirtualRealityBP/Blueprints/BP_MotionController` OtherActor))
  (if (== (`/Game/VirtualRealityBP/Blueprints/BP_MotionController.IndexFingerColli` _asbp_motion_controller) OtherComp)
    _))

(event `self.Pause_Box.OnComponentBeginOverlap`
  (params (OverlappedComponent :type "PrimitiveComponent Object Reference") (OtherActor :type "Actor Object Reference") (OtherComp :type "PrimitiveComponent Object Reference") (OtherBodyIndex :type Integer) (bFromSweep :type Boolean) (SweepResult :type "HitResult Structure (by ref)"))
  ;[1 1 1] Play/Pause
  (bind _asbp_motion_controller (cast `/Game/VirtualRealityBP/Blueprints/BP_MotionController` OtherActor))
  (if (and (== (`/Game/VirtualRealityBP/Blueprints/BP_MotionController.IndexFingerColli` _asbp_motion_controller) OtherComp) (not (`self.inputLock`)))
    (set `self.inputLock` true)
    (`/Game/CryoVR_GeneralContent/Blueprints/BPC_PlayBackController.PausePlayBack` (`/Game/CryoVR_GeneralContent/Blueprints/BP_PlayBackCharacter.BPC_PlayBackController` (`self.Player`)))
    (`KismetSystemLibrary.Delay` 0.5 :!label _label)
    (set `self.InputLock` false)))

(event `self.Play_Box.OnComponentBeginOverlap`
  (params (OverlappedComponent :type "PrimitiveComponent Object Reference") (OtherActor :type "Actor Object Reference") (OtherComp :type "PrimitiveComponent Object Reference") (OtherBodyIndex :type Integer) (bFromSweep :type Boolean) (SweepResult :type "HitResult Structure (by ref)"))
  ;[1 1 1] Play/Pause
  (bind _asbp_motion_controller (cast `/Game/VirtualRealityBP/Blueprints/BP_MotionController` OtherActor))
  (if (and (== (`/Game/VirtualRealityBP/Blueprints/BP_MotionController.IndexFingerColli` _asbp_motion_controller) OtherComp) (not (`self.inputLock`)))
    (set `self.inputLock` true)
    (`/Game/CryoVR_GeneralContent/Blueprints/BPC_PlayBackController.ContinuePlayBack` (`/Game/CryoVR_GeneralContent/Blueprints/BP_PlayBackCharacter.BPC_PlayBackController` (`self.Player`)))
    (goto _label)))

(event `self.Slow_Box.OnComponentBeginOverlap`
  (params (OverlappedComponent :type "PrimitiveComponent Object Reference") (OtherActor :type "Actor Object Reference") (OtherComp :type "PrimitiveComponent Object Reference") (OtherBodyIndex :type Integer) (bFromSweep :type Boolean) (SweepResult :type "HitResult Structure (by ref)"))
  ;[1 1 1] Slower/Faster
  (bind _asbp_motion_controller (cast `/Game/VirtualRealityBP/Blueprints/BP_MotionController` OtherActor))
  (if (and (== (`/Game/VirtualRealityBP/Blueprints/BP_MotionController.IndexFingerColli` _asbp_motion_controller) OtherComp) (not (`self.inputLock`)))
    (set `self.inputLock` true)
    (`/Game/CryoVR_GeneralContent/Blueprints/BPC_PlayBackController.SlowerPlay` (`/Game/CryoVR_GeneralContent/Blueprints/BP_PlayBackCharacter.BPC_PlayBackController` (`self.Player`)))
    (goto _label)))

(event `self.Fast_Box.OnComponentBeginOverlap`
  (params (OverlappedComponent :type "PrimitiveComponent Object Reference") (OtherActor :type "Actor Object Reference") (OtherComp :type "PrimitiveComponent Object Reference") (OtherBodyIndex :type Integer) (bFromSweep :type Boolean) (SweepResult :type "HitResult Structure (by ref)"))
  ;[1 1 1] Slower/Faster
  (bind _asbp_motion_controller (cast `/Game/VirtualRealityBP/Blueprints/BP_MotionController` OtherActor))
  (if (and (== (`/Game/VirtualRealityBP/Blueprints/BP_MotionController.IndexFingerColli` _asbp_motion_controller) OtherComp) (not (`self.inputLock`)))
    (set `self.inputLock` true)
    (`/Game/CryoVR_GeneralContent/Blueprints/BPC_PlayBackController.FasterPlay` (`/Game/CryoVR_GeneralContent/Blueprints/BP_PlayBackCharacter.BPC_PlayBackController` (`self.Player`)))
    (goto _label)))

(fn `UserConstructionScript`)